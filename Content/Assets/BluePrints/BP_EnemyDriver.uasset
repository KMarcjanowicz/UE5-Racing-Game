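; BP_EnemyDriver is an enemy race vehicle whose graph gates movement on the state of the race.
; Each Tick it halts movement while GameOverseer reports the race has not started.
; Once LapTimes reaches the overseer's lap limit and its last entry is non-zero, it applies the handbrake, then stops movement when forward speed is zero or below.
; The graph contains no steering or throttle logic.
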(event `self.ReceiveTick`
  (params (DeltaSeconds :type "Float (single-precision)"))
  (bind _vehiclemovement (`self.VehicleMovement`))
  (bind _laptimes (`self.LapTimes`))
  ;[1 1 1] Movement on/off depending on the state of the race.
  (if (`GameOverseer.bGameStart` (`self.GameOverseer`))
    ;[1 1 1] Check if last lap has it's time
    (if (>= (`KismetMathLibrary.Conv_IntToDouble` (+ (`KismetArrayLibrary.Array_LastIndex` (`self.LapTimes`)) 1)) (`KismetMathLibrary.Conv_IntToDouble` (`GameOverseer.MaxLaps` (`self.GameOverseer`))))
      (if (!= (`|GetArrayItem` _laptimes (`KismetArrayLibrary.Array_LastIndex` _laptimes)) 0.0)
        (`WheeledVehicleMovementComponent.SetHandbrakeInput` _vehiclemovement true)
        (if (<= (`WheeledVehicleMovementComponent.GetForwardSpeed` _vehiclemovement) 0.0)
          (`MovementComponent.StopMovementImmediately` (`self.GetMovementComponent`)))))
    (else
      (`MovementComponent.StopMovementImmediately` (`self.GetMovementComponent`)))))

(fn `UserConstructionScript`)